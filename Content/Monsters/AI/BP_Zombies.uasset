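; BP_Zombies is a zombie enemy that takes damage from mesh hits and dies when its health runs out.
; Health lives in BPActors, starts at 20, and is reduced through GetDamage when an actor implementing BP_Interface hits the mesh, with the new value printed.
; At zero health it flags itself dead, turns off capsule collision, detaches its controller and plays one of two death animations at random.
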(event OnComponentHit(Mesh)
  (params (HitComponent :type Primitive%20Component%20Object%20Reference) (OtherActor :type Actor%20Object%20Reference) (OtherComp :type Primitive%20Component%20Object%20Reference) (NormalImpulse :type Vector :default "0, 0, 0") (Hit :type Hit%20Result%20Structure%20%28by%20ref%29))
  (bind _bp_actors (Variables|Default|GetBP_Actors))
  (bind _bp_actors_2 (Variables|Default|GetBP_Actors))
  (bind _health (Variables|/Game/FirstPerson/Blueprints/BP_Actors.BP_Actors_C|GetHealth _bp_actors))
  (bind _returnvalue (> _health 0))
  (if (and (Utilities|DoesObjectImplementInterface OtherActor "/Game/FirstPerson/Blueprints/BP_Interface.BP_Interface_C") _returnvalue)
    (Utilities|FlowControl|Sequence
      (:then_0
        (Default|GetDamage _bp_actors_2 self)
        (Development|PrintString (Utilities|String|ToString(Integer) (Variables|/Game/FirstPerson/Blueprints/BP_Actors.BP_Actors_C|GetHealth _bp_actors_2))))
      (:then_1
        (if (not _returnvalue)
          (Variables|Default|SetisDead true)
          (Components|Activation|SetActive (Variables|Character|GetCharacterMovement) true false)
          (Collision|SetCollisionEnabled (Variables|Collision|GetCapsuleComponent) "NoCollision")
          (Collision|SetCollisionEnabled (Variables|Character|GetMesh) "QueryAndPhysics")
          (Class|Pawn|DetachfromControllerPendingDestroy)
          (if (Math|Random|RandomBool)
            (Components|Animation|PlayAnimation (Variables|Character|GetMesh) "/Game/Monsters/Animations/zombie_death.zombie_death" false)
            (else
              (Components|Animation|PlayAnimation (Variables|Character|GetMesh) "/Game/Monsters/Animations/zombie_dying.zombie_dying" false))))))))

(event EventBeginPlay
  (Variables|/Game/FirstPerson/Blueprints/BP_Actors.BP_Actors_C|SetHealth (Variables|Default|GetBP_Actors) 20))

(fn ConstructionScript)