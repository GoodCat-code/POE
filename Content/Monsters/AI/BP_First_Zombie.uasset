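; First zombie monster that turns toward and moves after the player while its Standing flag is set.
; Tick yaws the skeletal mesh to face the player character and issues a timed MoveComponentTo toward the pawn's X/Y, with no navigation or AI controller.
; BeginPlay binds to BP_Female's PlayerAway dispatcher, which sets the mesh's animation rate to normal speed when fired.
; Nothing here sets Standing.
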(event Custom|Player_Away_Event
  (Variables|/Script/Engine.SkeletalMeshComponent|SetGlobalAnimRateScale (Variables|SkeletalMeshActor|GetSkeletalMeshComponent) 1.0))

(event EventBeginPlay
  (Utilities|FlowControl|Sequence
    (:then_1
      (bind _returnvalue (Actor|GetActorOfClass "/Game/FirstPerson/Blueprints/BP_Female.BP_Female_C"))
      (EventDispatchers|AssignPlayerAway _returnvalue (delegate Custom|Player_Away_Event)))))

(event EventTick
  (params (DeltaSeconds :type Float%20%28single-precision%29))
  (bind _returnvalue (Game|Player|GetPlayerPawn 0))
  (bind _returnvalue_2 (Transformation|GetActorLocation _returnvalue))
  (if (Variables|Default|Getstanding)
    (Transformation|SetWorldRotation (Variables|SkeletalMeshActor|GetSkeletalMeshComponent) (Math|Rotator|MakeRotator 0.0 0.0 (+ (.yaw (Math|Rotator|FindLookatRotation (Transformation|GetWorldLocation (Variables|SkeletalMeshActor|GetSkeletalMeshComponent)) (Transformation|GetActorLocation (Game|GetPlayerCharacter 0)))) -9e+01)) false false)
    (Components|MoveComponentTo (Variables|SkeletalMeshActor|GetSkeletalMeshComponent) (Math|Vector|MakeVector (.x _returnvalue_2) (.y _returnvalue_2) 0.0) "0, 0, 0" false false 1e+01 false)))

(fn ConstructionScript)